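; BP_NPC is an AI-controlled enemy NPC that starts its controller's brain logic on BeginPlay, with ActivateEnemy able to start it again.
; A trigger component shows a popup widget while the player character overlaps it, and Tick rotates the widget to face the camera.
; DeactivateEnemy destroys the enemy scanner component once and sets a flag, but leaves the AI running, as its StopLogic and DestroyActor nodes are unwired.
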(event OnComponentBeginOverlap(WidgetTrigger)
  (params (OverlappedComponent :type Primitive%20Component%20Object%20Reference) (OtherActor :type Actor%20Object%20Reference) (OtherComp :type Primitive%20Component%20Object%20Reference) (OtherBodyIndex :type Integer) (bFromSweep :type Boolean) (SweepResult :type Hit%20Result%20Structure%20%28by%20ref%29))
  ;[1 1 1] Pop Up Text
  (Utilities|Casting|CastToBP_SV_PlayerCharacter OtherActor)
  (Rendering|SetVisibility (Variables|Default|GetWidget) true false))

(event OnComponentEndOverlap(WidgetTrigger)
  (params (OverlappedComponent :type Primitive%20Component%20Object%20Reference) (OtherActor :type Actor%20Object%20Reference) (OtherComp :type Primitive%20Component%20Object%20Reference) (OtherBodyIndex :type Integer))
  ;[1 1 1] Pop Up Text
  (Utilities|Casting|CastToBP_SV_PlayerCharacter OtherActor)
  (Rendering|SetVisibility (Variables|Default|GetWidget) false false))

(event EventBeginPlay
  (AI|Logic|StartLogic (Variables|/Script/AIModule.AIController|GetBrainComponent (AI|GetAIController self))))

(event Collision|EventActorBeginOverlap
  (params (OtherActor :type Actor%20Object%20Reference)))

(event EventTick
  (params (DeltaSeconds :type Float%20%28single-precision%29))
  ;[1 1 1] Pop Up Text
  (Transformation|SetWorldRotation (Variables|Default|GetWidget) (Math|Rotator|FindLookatRotation (Transformation|GetWorldLocation (Variables|Default|GetWidget)) (Transformation|GetWorldLocation (Variables|/Script/Engine.Actor|GetRootComponent (Game|GetPlayerCameraManager 0)))) false false))

(event EventDeactivateEnemy
  (if (not (Variables|Default|GetisDeactivated))
    (Components|DestroyComponent (Variables|Default|GetBP_SV_EnemyScanner))
    (Variables|Default|SetisDeactivated true)))

(fn ConstructionScript)

(fn ActivateEnemy
  (AI|Logic|StartLogic (Variables|/Script/AIModule.AIController|GetBrainComponent (AI|GetAIController self))))