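; Bomb baby enemy that counts down to an explosion or defusal and also controls the level's music.
; Tick drives a dial hand and countdown text from the explosion timer.
; OnExplode swaps in the broken mesh with sound and effects, while OnDefuse shows a smiley, kills the warning light and restores ambient music.
; Player-triggered collision boxes play the intro sting and start, stop or switch between ambient and action tracks.
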(event OnComponentBeginOverlap(AmbientCollisionBox6)
  (params (OverlappedComponent :type Primitive%20Component%20Object%20Reference) (OtherActor :type Actor%20Object%20Reference) (OtherComp :type Primitive%20Component%20Object%20Reference) (OtherBodyIndex :type Integer) (bFromSweep :type Boolean) (SweepResult :type Hit%20Result%20Structure%20%28by%20ref%29))
  (Utilities|Casting|CastToBP_SV_PlayerCharacter OtherActor)
  (Audio|Components|Audio|Play (Variables|Components|GetAction_Cue) 0.0)
  (Audio|Components|Audio|Stop (Variables|Components|GetAmbientMusic))
  (Collision|SetCollisionEnabled (Variables|Components|GetAmbientCollisionBox6) "NoCollision"))

(event OnComponentBeginOverlap(AmbientCollisionBox7)
  (params (OverlappedComponent :type Primitive%20Component%20Object%20Reference) (OtherActor :type Actor%20Object%20Reference) (OtherComp :type Primitive%20Component%20Object%20Reference) (OtherBodyIndex :type Integer) (bFromSweep :type Boolean) (SweepResult :type Hit%20Result%20Structure%20%28by%20ref%29))
  (Utilities|Casting|CastToBP_SV_PlayerCharacter OtherActor)
  (Audio|Components|Audio|Stop (Variables|Components|GetAmbientMusic))
  (Development|PrintText "Music Stopping"))

(event OnComponentBeginOverlap(AmbientCollisionBox9)
  (params (OverlappedComponent :type Primitive%20Component%20Object%20Reference) (OtherActor :type Actor%20Object%20Reference) (OtherComp :type Primitive%20Component%20Object%20Reference) (OtherBodyIndex :type Integer) (bFromSweep :type Boolean) (SweepResult :type Hit%20Result%20Structure%20%28by%20ref%29))
  (Utilities|Casting|CastToBP_SV_PlayerCharacter OtherActor)
  (Audio|Components|Audio|Stop (Variables|Components|GetAmbientMusic))
  (Development|PrintText "Music Stopping"))

(event OnComponentBeginOverlap(AmbientCollisionBox4)
  (params (OverlappedComponent :type Primitive%20Component%20Object%20Reference) (OtherActor :type Actor%20Object%20Reference) (OtherComp :type Primitive%20Component%20Object%20Reference) (OtherBodyIndex :type Integer) (bFromSweep :type Boolean) (SweepResult :type Hit%20Result%20Structure%20%28by%20ref%29))
  (Utilities|Casting|CastToBP_SV_PlayerCharacter OtherActor)
  (if (Audio|Components|Audio|IsPlaying (Variables|Components|GetAmbientMusic))
    (Development|PrintText "Music Already Playing")
    (else
      (Audio|Components|Audio|Play (Variables|Components|GetAmbientMusic) 0.0)
      (Development|PrintText "Playing Music"))))

(event OnComponentEndOverlap(AmbientCollisionBox9)
  (params (OverlappedComponent :type Primitive%20Component%20Object%20Reference) (OtherActor :type Actor%20Object%20Reference) (OtherComp :type Primitive%20Component%20Object%20Reference) (OtherBodyIndex :type Integer))
  (Utilities|Casting|CastToBP_SV_PlayerCharacter OtherActor)
  (Audio|Components|Audio|Stop (Variables|Components|GetAmbientMusic))
  (Development|PrintText "Music Stopping"))

(event OnComponentBeginOverlap(AmbientCollisionBox10)
  (params (OverlappedComponent :type Primitive%20Component%20Object%20Reference) (OtherActor :type Actor%20Object%20Reference) (OtherComp :type Primitive%20Component%20Object%20Reference) (OtherBodyIndex :type Integer) (bFromSweep :type Boolean) (SweepResult :type Hit%20Result%20Structure%20%28by%20ref%29))
  (Utilities|Casting|CastToBP_SV_PlayerCharacter OtherActor)
  (if (Audio|Components|Audio|IsPlaying (Variables|Components|GetAction_Cue))
    (Development|PrintText "Music Already Playing")
    (else
      (Audio|Components|Audio|Play (Variables|Components|GetAction_Cue) 0.0)
      (Development|PrintText "Playing Music"))))

(event OnComponentBeginOverlap(AmbientCollisionBox5)
  (params (OverlappedComponent :type Primitive%20Component%20Object%20Reference) (OtherActor :type Actor%20Object%20Reference) (OtherComp :type Primitive%20Component%20Object%20Reference) (OtherBodyIndex :type Integer) (bFromSweep :type Boolean) (SweepResult :type Hit%20Result%20Structure%20%28by%20ref%29))
  (Utilities|Casting|CastToBP_SV_PlayerCharacter OtherActor)
  (if (Audio|Components|Audio|IsPlaying (Variables|Components|GetAmbientMusic))
    (Development|PrintText "Music Already Playing")
    (else
      (Audio|Components|Audio|Play (Variables|Components|GetAmbientMusic) 0.0)
      (Development|PrintText "Playing Music"))))

(event OnComponentBeginOverlap(AmbientCollisionBox8)
  (params (OverlappedComponent :type Primitive%20Component%20Object%20Reference) (OtherActor :type Actor%20Object%20Reference) (OtherComp :type Primitive%20Component%20Object%20Reference) (OtherBodyIndex :type Integer) (bFromSweep :type Boolean) (SweepResult :type Hit%20Result%20Structure%20%28by%20ref%29))
  (Utilities|Casting|CastToBP_SV_PlayerCharacter OtherActor)
  (Audio|Components|Audio|Stop (Variables|Components|GetAmbientMusic))
  (Development|PrintText "Music Stopping"))

(event OnComponentBeginOverlap(AmbientCollisionBox1)
  (params (OverlappedComponent :type Primitive%20Component%20Object%20Reference) (OtherActor :type Actor%20Object%20Reference) (OtherComp :type Primitive%20Component%20Object%20Reference) (OtherBodyIndex :type Integer) (bFromSweep :type Boolean) (SweepResult :type Hit%20Result%20Structure%20%28by%20ref%29))
  (Utilities|Casting|CastToBP_SV_PlayerCharacter OtherActor)
  (if (Audio|Components|Audio|IsPlaying (Variables|Components|GetAmbientMusic))
    (Development|PrintText "Music Already Playing")
    (else
      (Audio|Components|Audio|Play (Variables|Components|GetAmbientMusic) 0.0)
      (Development|PrintText "Playing Music"))))

(event OnComponentBeginOverlap(AmbientCollisionBox2)
  (params (OverlappedComponent :type Primitive%20Component%20Object%20Reference) (OtherActor :type Actor%20Object%20Reference) (OtherComp :type Primitive%20Component%20Object%20Reference) (OtherBodyIndex :type Integer) (bFromSweep :type Boolean) (SweepResult :type Hit%20Result%20Structure%20%28by%20ref%29))
  (Utilities|Casting|CastToBP_SV_PlayerCharacter OtherActor)
  (if (Audio|Components|Audio|IsPlaying (Variables|Components|GetAmbientMusic))
    (Audio|Components|Audio|Stop (Variables|Components|GetAmbientMusic))
    (Audio|Components|Audio|Play (Variables|Components|GetFalling_Sting_Cue) 0.0)
    (Utilities|FlowControl|Delay 1.0)
    (Audio|Components|Audio|Play (Variables|Components|GetAction_Cue) 0.0)))

(event OnComponentBeginOverlap(AmbientCollisionBox)
  (params (OverlappedComponent :type Primitive%20Component%20Object%20Reference) (OtherActor :type Actor%20Object%20Reference) (OtherComp :type Primitive%20Component%20Object%20Reference) (OtherBodyIndex :type Integer) (bFromSweep :type Boolean) (SweepResult :type Hit%20Result%20Structure%20%28by%20ref%29))
  (Utilities|Casting|CastToBP_SV_PlayerCharacter OtherActor)
  (if (Audio|Components|Audio|IsPlaying (Variables|Components|GetAmbientMusic))
    (Development|PrintText "Music Already Playing")
    (else
      (Audio|Components|Audio|Play (Variables|Components|GetAmbientMusic) 0.0)
      (Development|PrintText "Playing Music"))))

(event OnComponentBeginOverlap(IntroMusicCollisionBox)
  (params (OverlappedComponent :type Primitive%20Component%20Object%20Reference) (OtherActor :type Actor%20Object%20Reference) (OtherComp :type Primitive%20Component%20Object%20Reference) (OtherBodyIndex :type Integer) (bFromSweep :type Boolean) (SweepResult :type Hit%20Result%20Structure%20%28by%20ref%29))
  (Utilities|Casting|CastToSV_PlayerCharacter OtherActor)
  (Collision|SetCollisionEnabled (Variables|Components|GetIntroMusicCollisionBox) "NoCollision")
  (Development|PrintText "Intro Sting Playing")
  (Audio|PlaySound2D "/Game/Steamwell_Sounds/Music/Start_Sting_Cue.Start_Sting_Cue" 1.0 1.0 0.0 0 0)
  (Utilities|FlowControl|Delay 18.0)
  (Audio|Components|Audio|Play (Variables|Components|GetAmbientMusic) 0.0))

(event OnComponentEndOverlap(AmbientCollisionBox7)
  (params (OverlappedComponent :type Primitive%20Component%20Object%20Reference) (OtherActor :type Actor%20Object%20Reference) (OtherComp :type Primitive%20Component%20Object%20Reference) (OtherBodyIndex :type Integer))
  (Utilities|Casting|CastToBP_SV_PlayerCharacter OtherActor)
  (Audio|Components|Audio|Stop (Variables|Components|GetAmbientMusic))
  (Development|PrintText "Music Stopping"))

(event OnComponentBeginOverlap(AmbientCollisionBox3)
  (params (OverlappedComponent :type Primitive%20Component%20Object%20Reference) (OtherActor :type Actor%20Object%20Reference) (OtherComp :type Primitive%20Component%20Object%20Reference) (OtherBodyIndex :type Integer) (bFromSweep :type Boolean) (SweepResult :type Hit%20Result%20Structure%20%28by%20ref%29))
  (Utilities|Casting|CastToBP_SV_PlayerCharacter OtherActor)
  (if (not (Audio|Components|Audio|IsPlaying (Variables|Components|GetAction_Cue)))
    (Audio|Components|Audio|Play (Variables|Components|GetAction_Cue) 0.0)
    (Development|PrintText "Playing Respawn Action")))

(event OnComponentEndOverlap(AmbientCollisionBox8)
  (params (OverlappedComponent :type Primitive%20Component%20Object%20Reference) (OtherActor :type Actor%20Object%20Reference) (OtherComp :type Primitive%20Component%20Object%20Reference) (OtherBodyIndex :type Integer))
  (Utilities|Casting|CastToBP_SV_PlayerCharacter OtherActor)
  (Audio|Components|Audio|Stop (Variables|Components|GetAmbientMusic))
  (Development|PrintText "Music Stopping"))

(event EventBeginPlay
  (Rendering|SetVisibility (Variables|Components|GetBrokenBaby) false false))

(event Collision|EventActorBeginOverlap
  (params (OtherActor :type Actor%20Object%20Reference)))

(event EventTick
  (params (DeltaSeconds :type Float%20%28single-precision%29))
  (bind _explosiontimerhandle (Variables|Default|GetExplosionTimerHandle))
  (bind _returnvalue (Class|KismetSystemLibrary|GetTimerElapsedTimeHandle _explosiontimerhandle))
  (Transformation|SetRelativeRotation (Variables|Components|Getbomb_baby_dial_hand) (Math|Rotator|MakeRotator 0.0 (Math|Float|MapRangeClamped _returnvalue 0.0 (Math|Conversions|ToFloat(Integer) (Variables|Default|GetTimeUntilExplosion)) -6e+01 6e+01) 0.0) false false)
  (if (> _returnvalue 0.0)
    (Rendering|Components|TextRender|SetText (Variables|Components|GetTextRender) (Utilities|Text|ToText(Float) (Utilities|Time|GetTimerRemainingTimebyHandle _explosiontimerhandle) "HalfToEven" false true 1 3 0 0))))

(event EventOnDefuse
  (Rendering|Components|TextRender|SetText (Variables|Components|GetTextRender) (Utilities|Text|ToText(String) ":D"))
  (Rendering|Components|Light|SetIntensity (Variables|Components|Getwarning) 0.0)
  (if (not (Audio|Components|Audio|IsPlaying (Variables|Components|GetAmbientMusic)))
    (Audio|Components|Audio|Play (Variables|Components|GetAmbientMusic) 0.0)
    (Audio|Components|Audio|Stop (Variables|Components|GetAction_Cue))))

(event EventOnExplode
  (Rendering|SetVisibility (Variables|Components|GetStaticMesh) false false)
  (Rendering|SetVisibility (Variables|Components|GetBrokenBaby) true false)
  (Audio|Components|Audio|Play (Variables|Components|GetBOOM_EXPLODE1_Cue) 0.0)
  (Components|Activation|Activate (Variables|Components|GetEXPLOSION) false)
  (Utilities|FlowControl|Delay 0.05)
  (Components|Activation|Deactivate (Variables|Components|GetEXPLOSION))
  (Components|Activation|Activate (Variables|Components|GetFireBOOM) false))

(fn ConstructionScript)

(fn GetAmbientAudioFR
  (return (Variables|Components|GetAmbientMusic)))