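; BP_Elevator is an interactable elevator that starts a one-time ride when the player character enters its trigger box.
; On first overlap by BP_SV_PlayerCharacter, it plays the elevator tune, sets a HasPlayed flag and runs the Elevator timeline to drive the Cube's relative location.
; When the timeline finishes, a ding sound plays; leaving the box only triggers a short delay with no further effect.
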(event OnComponentBeginOverlap(Box)
  (params (OverlappedComponent :type Primitive%20Component%20Object%20Reference) (OtherActor :type Actor%20Object%20Reference) (OtherComp :type Primitive%20Component%20Object%20Reference) (OtherBodyIndex :type Integer) (bFromSweep :type Boolean) (SweepResult :type Hit%20Result%20Structure%20%28by%20ref%29))
  (Utilities|Casting|CastToBP_SV_PlayerCharacter OtherActor)
  (if (not (Variables|Default|GethasPlayed))
    (Audio|PlaySoundatLocation "/Game/Steamwell_Sounds/Level3/elevator_tune_Cue.elevator_tune_Cue" "0, 0, 0" "0, 0, 0" 1.0 1.0 0.0 0 0 0 0)
    (Variables|Default|SethasPlayed true)
    (bind _elevator (Timeline|Elevator Play)
      (:Update
        (Transformation|SetRelativeLocation (Variables|Default|GetCube) _elevator false false))
      (:Finished
        (Audio|PlaySoundatLocation "/Game/Steamwell_Sounds/Sounds/Elevator_Ding.Elevator_Ding" "0, 0, 0" "0, 0, 0" 1.0 1.0 0.0 0 0 0 0)))))

(event OnComponentEndOverlap(Box)
  (params (OverlappedComponent :type Primitive%20Component%20Object%20Reference) (OtherActor :type Actor%20Object%20Reference) (OtherComp :type Primitive%20Component%20Object%20Reference) (OtherBodyIndex :type Integer))
  (Utilities|Casting|CastToBP_SV_PlayerCharacter OtherActor)
  (Utilities|FlowControl|Delay 0.2))

(event EventBeginPlay)

(event Collision|EventActorBeginOverlap
  (params (OtherActor :type Actor%20Object%20Reference)))

(event EventTick
  (params (DeltaSeconds :type Float%20%28single-precision%29)))

(fn ConstructionScript)