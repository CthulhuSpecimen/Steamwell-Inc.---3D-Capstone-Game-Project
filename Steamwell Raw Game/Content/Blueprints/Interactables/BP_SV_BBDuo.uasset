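; BP_SV_BBDuo is an interactable that rewards defusing a pair of bombs tracked by its BombBabyManagers.
; Each Tick it counts defused managers until exactly two are found.
; It then spawns an actor at the Plane component's location, activates the NSSteam effect and sets IsAttempted so the check fires only once.
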(event EventBeginPlay)

(event Collision|EventActorBeginOverlap
  (params (OtherActor :type Actor%20Object%20Reference)))

(event EventTick
  (params (DeltaSeconds :type Float%20%28single-precision%29))
  (Variables|Default|SetisDefusedCt 0)
  (if (not (Variables|Default|GetisAttempted))
    (for _array_element (Variables|Default|GetBombBabyManagers)
      (if (Variables|/Game/Blueprints/Interactables/BP_SV_PressurePlateManager_BB.BP_SV_PressurePlateManager_BB_C|GetisDefused _array_element)
        (Variables|Default|SetisDefusedCt (+ 1 (Variables|Default|GetisDefusedCt)))))
    (if (== (Variables|Default|GetisDefusedCt) 2)
      (Game|SpawnActorfromClass "/Game/Blueprints/Interactables/Gear/BP_SV_Gear.BP_SV_Gear_C" (Math|Conversions|ToTransform(Vector) (Transformation|GetWorldLocation (Variables|Default|GetPlane))) "AdjustIfPossibleButAlwaysSpawn" "MultiplyWithRoot" 0 0)
      (Variables|Default|SetisAttempted true)
      (Components|Activation|Activate (Variables|Default|GetNS_Steam) false))))

(fn ConstructionScript)