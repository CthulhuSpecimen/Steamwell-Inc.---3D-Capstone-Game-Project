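; BP_SV_Checkpoint is a checkpoint actor that saves the game when the player character overlaps it and activates the Bomb Baby linked to its ID.
; Overlap passes the player to SV_GameInstance's SaveGame, then asks SV_GameModeBase to activate the Bomb Baby.
; BeginPlay caches the player and runs the same activation check, covering respawns inside the checkpoint.
; The HasNotEntered flag prevents re-entry from adding another timer.
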(event EventBeginPlay
  ;[1 1 1] Activates Bomb Baby on Respawning
  (bind _asbp_sv_player_character (Utilities|Casting|CastToBP_SV_PlayerCharacter (Game|GetPlayerCharacter 0)))
  ;[1 1 1] Activates Bomb Baby
  ;;[1 1 1] Prevents adding another timer when reentering the checkpoint
  (if (and (Collision|IsOverlappingActor _asbp_sv_player_character :!class /Script/Engine.Actor) (Variables|Default|GetHasNotEntered))
    (bind _assv_game_mode_base (Utilities|Casting|CastToSV_GameModeBase (Game|GetGameMode)))
    (Class|SVGameModeBase|ActivateBombBaby _assv_game_mode_base (Variables|BombBaby|GetID))
    (Variables|Default|SetHasNotEntered false)))

(event Collision|EventActorBeginOverlap
  (params (OtherActor :type Actor%20Object%20Reference))
  (bind _asbp_sv_player_character (Utilities|Casting|CastToBP_SV_PlayerCharacter OtherActor)
    (:then
      (bind _assv_game_instance (Utilities|Casting|CastToSV_GameInstance (Game|GetGameInstance))
        (:then
          (Class|SVGameInstance|SaveGame _assv_game_instance _asbp_sv_player_character)
          ;[1 1 1] Activates Bomb Baby
          ;;[1 1 1] Prevents adding another timer when reentering the checkpoint
          (if (and (Collision|IsOverlappingActor (stale EventBeginPlay _asbp_sv_player_character) :!class /Script/Engine.Actor) (Variables|Default|GetHasNotEntered))
            (bind _assv_game_mode_base (Utilities|Casting|CastToSV_GameModeBase (Game|GetGameMode)))
            (Class|SVGameModeBase|ActivateBombBaby _assv_game_mode_base (Variables|BombBaby|GetID))
            (Variables|Default|SetHasNotEntered false)))
        (:CastFailed
          (Development|PrintString "failr" :!label _label))))
    (:CastFailed
      (goto _label))))

(event EventTick
  (params (DeltaSeconds :type Float%20%28single-precision%29)))

(fn ConstructionScript)