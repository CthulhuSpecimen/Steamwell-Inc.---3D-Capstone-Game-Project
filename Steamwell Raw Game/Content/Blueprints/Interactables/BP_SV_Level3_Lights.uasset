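; Level 3 light sequence actor that cycles four cylinder meshes through lit and unlit materials with a ping sound for each step.
; BeginPlay runs an endless loop of one-second delays, lighting each cylinder in turn while switching the previous one off.
; After the last cylinder turns off, the chain wires back to the start, so the chase pattern repeats without Tick or timers.
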(event EventBeginPlay
  (Utilities|FlowControl|Delay 1.0 :!label _label)
  (Audio|Components|Audio|Play (Variables|Default|GetPing1) 0.0)
  (Rendering|Material|SetMaterial (Variables|Default|GetCylinder) 0 "/Game/LightOn.LightOn")
  (Utilities|FlowControl|Delay 1.0)
  (Audio|Components|Audio|Play (Variables|Default|GetPing2) 0.0)
  (Rendering|Material|SetMaterial (Variables|Default|GetCylinder1) 0 "/Game/LightOn.LightOn")
  (Rendering|Material|SetMaterial (Variables|Default|GetCylinder) 0 "/Game/Materials/LightOff.LightOff")
  (Utilities|FlowControl|Delay 1.0)
  (Audio|Components|Audio|Play (Variables|Default|GetPing3) 0.0)
  (Rendering|Material|SetMaterial (Variables|Default|GetCylinder2) 0 "/Game/LightOn.LightOn")
  (Rendering|Material|SetMaterial (Variables|Default|GetCylinder1) 0 "/Game/Materials/LightOff.LightOff")
  (Utilities|FlowControl|Delay 1.0)
  (Audio|Components|Audio|Play (Variables|Default|GetPing4) 0.0)
  (Rendering|Material|SetMaterial (Variables|Default|GetCylinder3) 0 "/Game/LightOn.LightOn")
  (Rendering|Material|SetMaterial (Variables|Default|GetCylinder2) 0 "/Game/Materials/LightOff.LightOff")
  (Utilities|FlowControl|Delay 1.0)
  (Rendering|Material|SetMaterial (Variables|Default|GetCylinder3) 0 "/Game/Materials/LightOff.LightOff")
  (goto _label))

(event Collision|EventActorBeginOverlap
  (params (OtherActor :type Actor%20Object%20Reference)))

(event EventTick
  (params (DeltaSeconds :type Float%20%28single-precision%29)))

(fn ConstructionScript)