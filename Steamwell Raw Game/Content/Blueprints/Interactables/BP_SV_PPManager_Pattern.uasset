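; Manager for a pipe-and-plate pattern puzzle that rewards a gear or, if flagged final, calls OnEnemyDefeat.
; BeginPlay records pipe start locations and, if flashing is enabled, starts a looping timer that flashes the lights in sequence as Increase cycles an index.
; PlatesComplete stops steam, turns lights green and spawns the gear once.
; PlatesRejected sounds alarms, flashes red, clears player pushing and resets pipes and plates.
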(event EventBeginPlay
  (for _array_element (Variables|Default|GetPatternPipes)
    (Utilities|Array|Add (Variables|Default|GetInitialLoc) (Transformation|GetActorLocation _array_element))
    (if (Variables|Default|GetisFlash)
      (bind _returnvalue (Utilities|Time|SetTimerbyFunctionName 0 "increase" 3.0 true))
      (Variables|Default|SetloopTimer _returnvalue)))
  (Development|PrintString "locations added"))

(event Collision|EventActorBeginOverlap
  (params (OtherActor :type Actor%20Object%20Reference)))

(event EventTick
  (params (DeltaSeconds :type Float%20%28single-precision%29)))

(event EventPlatesComplete
  (Development|PrintString "COMPLETE")
  (Development|PrintString "POOF" true true "(R=0.794931,G=0.040544,B=1.000000,A=1.000000)")
  (if (Variables|Default|GetisFinal)
    (Default|CallOnEnemyDefeat)
    (elif (not (Variables|Default|GetisComplete))
      (Components|Activation|Activate (Variables|Default|GetNS_Steam) false)
      (Rendering|Components|Light|SetLightColor (Variables|Default|GetRectLight) (Math|Color|MakeColor 0.0 1.0 0.0) true)
      (Rendering|Components|Light|SetLightColor (Variables|Default|GetRectLight2) (Math|Color|MakeColor 0.0 1.0 0.0) true)
      (Rendering|Components|Light|SetLightColor (Variables|Default|GetRectLight3) (Math|Color|MakeColor 0.0 1.0 0.0) true)
      (Rendering|Components|Light|SetLightColor (Variables|Default|GetRectLight4) (Math|Color|MakeColor 0.0 1.0 0.0) true)
      (Rendering|Components|Light|SetLightColor (Variables|Default|GetRectLight1) (Math|Color|MakeColor 0.0 1.0 0.0) true)
      (Game|SpawnActorfromClass "/Game/Blueprints/Interactables/Gear/BP_SV_Gear.BP_SV_Gear_C" (Math|Conversions|ToTransform(Vector) (Transformation|GetWorldLocation (Variables|Default|GetPlane))) "AdjustIfPossibleButAlwaysSpawn" "MultiplyWithRoot" 0 0)
      (Audio|PlaySoundatLocation "/Game/Steamwell_Sounds/Sound_Cues/puzzle_complete_Cue.puzzle_complete_Cue" "0, 0, 0" "0, 0, 0" 1.0 1.0 0.0 0 0 0 0)
      (Variables|Default|SetisComplete true))))

(event EventPlatesRejected
  (Utilities|FlowControl|Sequence
    (:then_0
      (Audio|PlaySoundatLocation "/Game/Steamwell_Sounds/Sounds/machine_error3.machine_error3" "0, 0, 0" "0, 0, 0" 1.0 1.0 0.0 0 0 0 0)
      (Audio|PlaySoundatLocation "/Game/Steamwell_Sounds/Level2_Sounds/pipe_lock_fail.pipe_lock_fail" "0, 0, 0" "0, 0, 0" 1.0 1.0 0.0 0 0 0 0)
      (Development|PrintString "NOT COMPLETE" true true "(R=1.000000,G=0.000000,B=0.071324,A=1.000000)")
      (bind _assv_player_character (Utilities|Casting|CastToSV_PlayerCharacter (Game|GetPlayerCharacter 0)))
      (Variables|/Script/Steamwell.SV_PlayerCharacter|SetisPushing _assv_player_character false)
      (for (_array_element _array_index) (Variables|Default|GetPatternPipes)
        (Transformation|SetActorLocation _array_element (Utilities|Array|Get(acopy) (Variables|Default|GetInitialLoc) _array_index) false false)
        (Variables|/Script/Steamwell.SV_PushableObject|SetisPlaced _array_element false)
        (for _array_element_2 (Variables|Default|GetPatternPlates)
          (Variables|/Script/Steamwell.SV_PressurePlate|SetisPlaced _array_element_2 false))))
    (:then_1
      (Audio|PlaySoundatLocation "/Game/Steamwell_Sounds/Sounds/AlarmPatternFail_Cue.AlarmPatternFail_Cue" "0, 0, 0" "0, 0, 0" 1.0 1.0 0.0 0 0 0 0)
      (Rendering|Components|Light|SetLightColor (Variables|Default|GetRectLight) (Math|Color|MakeColor 1.0 0.0 0.0) true)
      (Rendering|Components|Light|SetLightColor (Variables|Default|GetRectLight2) (Math|Color|MakeColor 1.0 0.0 0.0) true)
      (Rendering|Components|Light|SetLightColor (Variables|Default|GetRectLight3) (Math|Color|MakeColor 1.0 0.0 0.0) true)
      (Rendering|Components|Light|SetLightColor (Variables|Default|GetRectLight4) (Math|Color|MakeColor 1.0 0.0 0.0) true)
      (Rendering|Components|Light|SetLightColor (Variables|Default|GetRectLight1) (Math|Color|MakeColor 1.0 0.0 0.0) true)
      (Utilities|FlowControl|Delay 1.5)
      (Rendering|Components|Light|SetLightColor (Variables|Default|GetRectLight2) (Math|Color|MakeColor 0.323143 0.171441 0.035601) true))))

(fn ConstructionScript)

(fn Increase
  (if (== (Variables|Default|Getiterator) (Utilities|Array|Length (Variables|Default|GetLights)))
    (Variables|Default|Setiterator 0))
  (Default|FlashLight (Utilities|Array|Get(acopy) (Variables|Default|GetLights) (Variables|Default|Getiterator)))
  (bind _result (Math|Integer|IncrementInt (Variables|Default|Getiterator))
    (:%20%20
      (Variables|Default|Setiterator _result))))