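; BP_SV_PipeSpin is an interactable that reacts to a pushable object overlapping it, apparently a pipe or crank on a machine.
; On overlap with an SV_PushableObject, it stores that object's world yaw, plays the PipeOnMachine audio and switches its mesh to a lit material.
; Any overlap ending, without a type check, restores the unlit material and prints debug text.
; The stored yaw is not read here, and no spin logic is present.
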(event EventBeginPlay)

(event Collision|EventActorBeginOverlap
  (params (OtherActor :type Actor%20Object%20Reference))
  (bind _assv_pushable_object (Utilities|Casting|CastToSV_PushableObject OtherActor))
  (Variables|Default|SetOrigDegr (.Yaw (Math|Rotator|BreakRotator (Transformation|GetWorldRotation (Variables|/Script/Steamwell.SV_PushableObject|GetMeshComponent _assv_pushable_object)))))
  (Audio|Components|Audio|Play (Variables|Default|GetPipe_On_Machine) 0.0)
  (Rendering|Material|SetMaterial (Variables|Character|GetMesh) 0 "/Game/Materials/LightOn.LightOn"))

(event Collision|EventActorEndOverlap
  (params (OtherActor :type Actor%20Object%20Reference))
  (Development|PrintText "CrankEndOverlap")
  (Rendering|Material|SetMaterial (Variables|Character|GetMesh) 0 "/Game/Materials/LightOff.LightOff"))

(fn ConstructionScript)