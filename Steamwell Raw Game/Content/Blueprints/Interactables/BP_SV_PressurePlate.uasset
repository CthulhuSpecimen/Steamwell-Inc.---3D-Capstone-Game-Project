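; Pressure plate interactable that reacts when a pushable block is placed on it.
; Its BlockPlaced event teleports the pushed object to the plate's X and Y while keeping the object's height, then deactivates the Niagara effect and plays a pipe lock sound.
; The graph contains no overlap detection, and a node setting the mesh collision to BlockAll is left unconnected.
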(event EventBeginPlay)

(event Collision|EventActorBeginOverlap
  (params (OtherActor :type Actor%20Object%20Reference)))

(event EventTick
  (params (DeltaSeconds :type Float%20%28single-precision%29)))

(event EventBlockPlaced
  (params (PushedObject :type SV%20Pushable%20Object%20Object%20Reference))
  (bind _returnvalue (Transformation|GetActorLocation))
  (bind (_x _y) (Math|Vector|BreakVector _returnvalue))
  (Transformation|SetActorLocation PushedObject (Math|Vector|MakeVector _x _y (.Z (Math|Vector|BreakVector (Transformation|GetActorLocation PushedObject)))) false false)
  (Components|Activation|Deactivate (Variables|Default|GetNiagara))
  (Audio|PlaySoundatLocation "/Game/Steamwell_Sounds/Sound_Cues/pipe_lock_Cue.pipe_lock_Cue" "0, 0, 0" "0, 0, 0" 1.0 1.0 0.0 0 0 0 0))

(fn ConstructionScript)