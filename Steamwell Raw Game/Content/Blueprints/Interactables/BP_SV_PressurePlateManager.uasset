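; Pressure plate puzzle manager that hands out the reward when the plates are completed.
; Its PlatesComplete event activates a steam effect, spawns a BP_SV_Gear at the Plane component, plays a completion sound at world origin and turns the RectLight green, alongside a debug print.
; The Blueprint runs no plate detection of its own, so completion relies on an external call to that event.
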(event EventBeginPlay)

(event EventTick
  (params (DeltaSeconds :type Float%20%28single-precision%29)))

(event EventPlatesComplete
  (Development|PrintString "POOF" true true "(R=0.794931,G=0.040544,B=1.000000,A=1.000000)")
  (Components|Activation|Activate (Variables|Default|GetNS_Steam) false)
  (Game|SpawnActorfromClass "/Game/Blueprints/Interactables/Gear/BP_SV_Gear.BP_SV_Gear_C" (Math|Conversions|ToTransform(Vector) (Transformation|GetWorldLocation (Variables|Default|GetPlane))) "AdjustIfPossibleButAlwaysSpawn" "MultiplyWithRoot" 0 0)
  (Audio|PlaySoundatLocation "/Game/Steamwell_Sounds/Sound_Cues/puzzle_complete_Cue.puzzle_complete_Cue" "0, 0, 0" "0, 0, 0" 1.0 1.0 0.0 0 0 0 0)
  (Rendering|Components|Light|SetLightColor (Variables|Default|GetRectLight) (Math|Color|MakeColor 0.0 1.0 0.0) true))

(fn ConstructionScript)