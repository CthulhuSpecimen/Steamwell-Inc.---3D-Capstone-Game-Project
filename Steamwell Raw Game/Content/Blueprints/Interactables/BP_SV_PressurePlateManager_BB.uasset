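; Pressure plate manager that defuses a Bomb Baby when its plates are complete.
; PlatesComplete tells SV_GameModeBase to defuse the matching BombBabyID, marks itself defused, spawns an actor at the Plane component's location and activates the steam effect.
; A duo check that would hold the spawn until every Bomb Baby is defused is left disconnected, so the spawn follows each completion directly.
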(event EventBeginPlay
  (Variables|Default|SetisComplete true))

(event Collision|EventActorBeginOverlap
  (params (OtherActor :type Actor%20Object%20Reference)))

(event EventTick
  (params (DeltaSeconds :type Float%20%28single-precision%29)))

(event EventPlatesComplete
  (bind _assv_game_mode_base (Utilities|Casting|CastToSV_GameModeBase (Game|GetGameMode)))
  (Class|SVGameModeBase|DefuseBombBaby _assv_game_mode_base (Variables|Default|GetBombBabyID))
  (Variables|Default|SetisDefused true)
  (Game|SpawnActorfromClass "/Game/Blueprints/Interactables/Gear/BP_SV_Gear.BP_SV_Gear_C" (Math|Conversions|ToTransform(Vector) (Transformation|GetWorldLocation (Variables|Default|GetPlane))) "AdjustIfPossibleButAlwaysSpawn" "MultiplyWithRoot" 0 0)
  (Components|Activation|Activate (Variables|Default|GetNS_Steam) false))

(fn ConstructionScript)