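; Signal light interactable that lights up once when play begins, then switches off.
; On BeginPlay, FlashLight swaps the Light component to the LightOn material and starts a named-function timer.
; When the timer fires two seconds later, TurnOffLight applies the LightOff material and clears the stored timer handle.
; Despite the flash naming, nothing re-triggers it, so it does not blink repeatedly.
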(event EventBeginPlay
  (CallFunction|FlashLight))

(event Collision|EventActorBeginOverlap
  (params (OtherActor :type Actor%20Object%20Reference)))

(event EventTick
  (params (DeltaSeconds :type Float%20%28single-precision%29)))

(fn ConstructionScript)

(fn FlashLight
  (Rendering|Material|SetMaterial (Variables|Default|GetLight) 0 "/Game/LightOn.LightOn")
  (bind _returnvalue (Utilities|Time|SetTimerbyFunctionName 0 "TurnOffLight" 2.0))
  (Variables|Default|SetturnOff _returnvalue))

(fn TurnOffLight
  (Rendering|Material|SetMaterial (Variables|Default|GetLight) 0 "/Game/Materials/LightOff.LightOff")
  (Utilities|Time|ClearandInvalidateTimerbyHandle (Variables|Default|GetturnOff)))