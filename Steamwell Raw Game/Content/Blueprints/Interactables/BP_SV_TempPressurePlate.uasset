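; A temporary one-shot pressure plate interactable that spawns a gear when an actor tagged "cart" overlaps it.
; The first cart overlap prints a debug message, spawns BP_SV_Gear at a hardcoded world location, plays a machine sound at world origin and locks the plate.
; A separate trigger shows a pop-up widget while the player character is inside it, and Tick rotates that widget to face the camera.
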(event OnComponentBeginOverlap(WidgetTrigger)
  (params (OverlappedComponent :type Primitive%20Component%20Object%20Reference) (OtherActor :type Actor%20Object%20Reference) (OtherComp :type Primitive%20Component%20Object%20Reference) (OtherBodyIndex :type Integer) (bFromSweep :type Boolean) (SweepResult :type Hit%20Result%20Structure%20%28by%20ref%29))
  ;[1 1 1] Pop Up Text
  (Utilities|Casting|CastToBP_SV_PlayerCharacter OtherActor)
  (Rendering|SetVisibility (Variables|Default|GetWidget) true false))

(event OnComponentEndOverlap(WidgetTrigger)
  (params (OverlappedComponent :type Primitive%20Component%20Object%20Reference) (OtherActor :type Actor%20Object%20Reference) (OtherComp :type Primitive%20Component%20Object%20Reference) (OtherBodyIndex :type Integer))
  ;[1 1 1] Pop Up Text
  (Utilities|Casting|CastToBP_SV_PlayerCharacter OtherActor)
  (Rendering|SetVisibility (Variables|Default|GetWidget) false false))

(event EventBeginPlay
  (Variables|Default|SetplateUsed false))

(event Collision|EventActorBeginOverlap
  (params (OtherActor :type Actor%20Object%20Reference))
  (if (not (Variables|Default|GetplateUsed))
    (if (Actor|ActorHasTag OtherActor "cart")
      (Development|PrintString "POOF" true true "(R=0.794931,G=0.040544,B=1.000000,A=1.000000)")
      (Game|SpawnActorfromClass "/Game/Blueprints/Interactables/Gear/BP_SV_Gear.BP_SV_Gear_C" (Math|Conversions|ToTransform(Vector) "1850.000000,-1270.000000,90.000000") "AdjustIfPossibleButAlwaysSpawn" "MultiplyWithRoot" 0 0)
      (Audio|PlaySoundatLocation "/Game/Steamwell_Sounds/Sound_Cues/machine_move1_Cue.machine_move1_Cue" "0, 0, 0" "0, 0, 0" 1.0 1.0 0.0 0 0 0 0)
      (Variables|Default|SetplateUsed true))))

(event EventTick
  (params (DeltaSeconds :type Float%20%28single-precision%29))
  ;[1 1 1] Pop Up Text
  (Transformation|SetWorldRotation (Variables|Default|GetWidget) (Math|Rotator|FindLookatRotation (Transformation|GetWorldLocation (Variables|Default|GetWidget)) (Transformation|GetWorldLocation (Variables|/Script/Engine.Actor|GetRootComponent (Game|GetPlayerCameraManager 0)))) false false))

(fn ConstructionScript)