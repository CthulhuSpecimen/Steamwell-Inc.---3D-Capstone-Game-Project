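; Optimization actor for Level 5 that switches the area's particle effects on and off as the player moves through.
; Overlap of ActivateBox or DeactivateBox by BP_SV_PlayerCharacter activates or deactivates a fixed set of emitter components, including fire, sparks and smoke, and prints a debug message.
; Each box then disables its own collision and nothing here re-enables it, so each switch fires only once.
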(event OnComponentBeginOverlap(ActivateBox)
  (params (OverlappedComponent :type Primitive%20Component%20Object%20Reference) (OtherActor :type Actor%20Object%20Reference) (OtherComp :type Primitive%20Component%20Object%20Reference) (OtherBodyIndex :type Integer) (bFromSweep :type Boolean) (SweepResult :type Hit%20Result%20Structure%20%28by%20ref%29))
  (Utilities|Casting|CastToBP_SV_PlayerCharacter OtherActor)
  (Components|Activation|Activate (Variables|Default|GetNiagara) false)
  (Components|Activation|Activate (Variables|Default|GetNiagara1) false)
  (Components|Activation|Activate (Variables|Default|GetNiagara2) false)
  (Components|Activation|Activate (Variables|Default|GetNiagara3) false)
  (Components|Activation|Activate (Variables|Default|GetNiagara4) false)
  (Components|Activation|Activate (Variables|Default|GetCampFire1) false)
  (Components|Activation|Activate (Variables|Default|GetCampFire2) false)
  (Components|Activation|Activate (Variables|Default|GetPipeFire) false)
  (Components|Activation|Activate (Variables|Default|GetPipeFire1) false)
  (Components|Activation|Activate (Variables|Default|GetSparks1) false)
  (Components|Activation|Activate (Variables|Default|GetSparks2) false)
  (Components|Activation|Activate (Variables|Default|GetNS_Smoke1) false)
  (Components|Activation|Activate (Variables|Default|GetNS_Smoke) false)
  (Development|PrintString "Level 5 Activated")
  (Collision|SetCollisionEnabled (Variables|Default|GetActivate%20Box) "NoCollision"))

(event OnComponentBeginOverlap(DeactivateBox)
  (params (OverlappedComponent :type Primitive%20Component%20Object%20Reference) (OtherActor :type Actor%20Object%20Reference) (OtherComp :type Primitive%20Component%20Object%20Reference) (OtherBodyIndex :type Integer) (bFromSweep :type Boolean) (SweepResult :type Hit%20Result%20Structure%20%28by%20ref%29))
  (Utilities|Casting|CastToBP_SV_PlayerCharacter OtherActor)
  (Components|Activation|Deactivate (Variables|Default|GetNiagara))
  (Components|Activation|Deactivate (Variables|Default|GetNiagara1))
  (Components|Activation|Deactivate (Variables|Default|GetNiagara2))
  (Components|Activation|Deactivate (Variables|Default|GetNiagara3))
  (Components|Activation|Deactivate (Variables|Default|GetNiagara4))
  (Components|Activation|Deactivate (Variables|Default|GetCampFire1))
  (Components|Activation|Deactivate (Variables|Default|GetCampFire2))
  (Components|Activation|Deactivate (Variables|Default|GetPipeFire))
  (Components|Activation|Deactivate (Variables|Default|GetPipeFire1))
  (Components|Activation|Deactivate (Variables|Default|GetSparks1))
  (Components|Activation|Deactivate (Variables|Default|GetSparks2))
  (Components|Activation|Deactivate (Variables|Default|GetNS_Smoke))
  (Components|Activation|Deactivate (Variables|Default|GetNS_Smoke1))
  (Development|PrintString "Level 5 Deactivated")
  (Collision|SetCollisionEnabled (Variables|Default|GetDeactivate%20Box) "NoCollision"))

(event EventBeginPlay)

(event Collision|EventActorBeginOverlap
  (params (OtherActor :type Actor%20Object%20Reference)))

(event EventTick
  (params (DeltaSeconds :type Float%20%28single-precision%29)))

(fn ConstructionScript)