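; Player character Blueprint that adds the HUD, look-based interaction and a pause menu.
; A fast looping timer sphere-traces from the follow camera, tracking the BPI_Tutorial actor in view as TraceItem and toggling its trace state; left mouse sends it InteractMessage.
; IA_Pause toggles the pause widget, game pause, input mode and cursor.
; CheckInactivity runs on a timer but is empty; the WASD prompt logic is disconnected.
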(event Custom|CheckInactivity)

(event Custom|Create%20Interaction%20Trace
  (CallFunction|InteractionTrace))

(event Input|EnhancedActionEvents|EnhancedInputActionIA_Pause
  (params (ActionValue :type Boolean) (ElapsedSeconds :type Float%20%28double-precision%29) (TriggeredSeconds :type Float%20%28double-precision%29) (InputAction :type Input%20Action%20Object%20Reference :default "/Game/Input/Player/IA_Pause.IA_Pause"))
  (bind _returnvalue (Game|GetPlayerController 0))
  ;[1 1 1] Pause Menu
  (:Started
    (if (not (Variables|Default|GetIsPauseMenuOpen?))
      (Variables|Default|SetIsPauseMenuOpen? true)
      (bind _returnvalue_2 (UserInterface|CreateWidget "/Game/UI/Menu_UI/WB_PauseMenu.WB_PauseMenu_C" _returnvalue))
      (bind _output_get (Variables|Default|SetPause%20Menu%20Widget _returnvalue_2))
      (UserInterface|Viewport|AddtoViewport _output_get 0)
      (Input|SetInputModeGameandUI _returnvalue (Variables|Default|GetPause%20Menu%20Widget) "DoNotLock" true false)
      (Variables|/Script/Engine.PlayerController|SetbShowMouseCursor (Game|GetPlayerController 0) true)
      (Game|SetGamePaused true)
      (else
        (Variables|Default|SetIsPauseMenuOpen? false)
        (Widget|RemovefromParent (Variables|Default|GetPause%20Menu%20Widget))
        (Game|SetGamePaused false)
        (Input|SetInputModeGameOnly _returnvalue false)
        (Variables|/Script/Engine.PlayerController|SetbShowMouseCursor (Game|GetPlayerController 0) false)))))

(event EventBeginPlay
  (Utilities|Time|SetTimerbyFunctionName 0 "CheckInactivity" 1.0 true)
  (bind _returnvalue (Utilities|Time|SetTimerbyFunctionName 0 "Create Interaction Trace" 0.01 true))
  (Variables|Default|SetInteraction%20Timer _returnvalue)
  (bind _returnvalue_2 (UserInterface|CreateWidget "/Game/UI/PopupTexts/UI_HUD.UI_HUD_C"))
  (UserInterface|Viewport|AddtoViewport _returnvalue_2 0))

(event Collision|EventActorBeginOverlap
  (params (OtherActor :type Actor%20Object%20Reference)))

(event EventTick
  (params (DeltaSeconds :type Float%20%28single-precision%29)))

(event Input|MouseEvents|LeftMouseButton
  (params (Key :type Key%20Structure :default "None"))
  (:Pressed
    (Class|BPITutorial|Interact(Message) (Variables|Default|GetTrace%20Item))))

(fn ConstructionScript)

(fn InteractionTrace
  (bind _followcamera (Variables|Default|GetFollowCamera))
  (bind _returnvalue (Transformation|GetWorldLocation _followcamera))
  ;[1 1 1] Level 1 Tutorial
  (bind _outhit (Collision|SphereTraceByChannel _returnvalue (+ _returnvalue (* (Math|Vector|GetForwardVector (Transformation|GetWorldRotation _followcamera)) 1e+03)) 3.0 "TraceTypeQuery1" false 0 "None"))
  (if (Utilities|DoesObjectImplementInterface (.HitActor (Collision|BreakHitResult _outhit)) "/Game/UI/PopupTexts/BPI_Tutorial.BPI_Tutorial_C")
    (if (!= (.HitActor (Collision|BreakHitResult _outhit)) (Variables|Default|GetTrace%20Item))
      (bind _output_get (Variables|Default|SetTrace%20Item (.HitActor (Collision|BreakHitResult _outhit))))
      (Class|BPITutorial|CanReceiveTrace(Message) _output_get true))
    (else
      (Class|BPITutorial|CanReceiveTrace(Message) (Variables|Default|GetTrace%20Item) false)
      (Variables|Default|SetTrace%20Item 0))))