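; Level 5 bomb actor with two trigger boxes that react only to the player character.
; Entering BoxPing starts a looping timer that repeatedly plays a ping sound as a warning.
; Entering Box pauses that timer, plays the explosion and failure sounds, and briefly flashes a red effect.
; Each box disables its own collision once triggered, so both stages fire only once.
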(event OnComponentBeginOverlap(Box)
  (params (OverlappedComponent :type Primitive%20Component%20Object%20Reference) (OtherActor :type Actor%20Object%20Reference) (OtherComp :type Primitive%20Component%20Object%20Reference) (OtherBodyIndex :type Integer) (bFromSweep :type Boolean) (SweepResult :type Hit%20Result%20Structure%20%28by%20ref%29))
  (Utilities|Casting|CastToBP_SV_PlayerCharacter OtherActor)
  (Utilities|Time|PauseTimerbyHandle (stale OnComponentBeginOverlap(BoxPing) _returnvalue))
  (Audio|Components|Audio|Play (Variables|Default|GetBOOM) 0.0)
  (Audio|Components|Audio|Play (Variables|Default|GetBomb_Fail) 0.0)
  (Collision|SetCollisionEnabled (Variables|Default|GetBox) "NoCollision")
  (Components|Activation|Activate (Variables|Default|GetP_Flash01_Red_2) false)
  (Utilities|FlowControl|Delay 0.05)
  (Components|Activation|Deactivate (Variables|Default|GetP_Flash01_Red_2)))

(event OnComponentBeginOverlap(BoxPing)
  (params (OverlappedComponent :type Primitive%20Component%20Object%20Reference) (OtherActor :type Actor%20Object%20Reference) (OtherComp :type Primitive%20Component%20Object%20Reference) (OtherBodyIndex :type Integer) (bFromSweep :type Boolean) (SweepResult :type Hit%20Result%20Structure%20%28by%20ref%29))
  (Utilities|Casting|CastToBP_SV_PlayerCharacter OtherActor)
  (Collision|SetCollisionEnabled (Variables|Default|GetBoxPing) "NoCollision")
  (bind _returnvalue (Utilities|Time|SetTimerbyFunctionName 0 "BombPingEvent" 1.1 true)))

(event Custom|BombPingEvent
  (Audio|Components|Audio|Play (Variables|Default|GetBombPing) 0.0))

(event EventBeginPlay)

(event Collision|EventActorBeginOverlap
  (params (OtherActor :type Actor%20Object%20Reference)))

(event EventTick
  (params (DeltaSeconds :type Float%20%28single-precision%29)))

(fn ConstructionScript)